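; Ammo purchase Blueprint, a child class, that sells reserve ammo to a ThirdPersonCharacter for 200 points of Killcount.
; Box overlap checks the points, then adds PickupAmmo to the equipped weapon's MaxAmmo, capped at 360, and deducts the cost.
; Insufficient points or full ammo only print a French message.
; The reload sound plays at world origin, only when the refill reaches the cap.
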(event OnComponentBeginOverlap(Box)
  (params (OverlappedComponent :type Primitive%20Component%20Object%20Reference) (OtherActor :type Actor%20Object%20Reference) (OtherComp :type Primitive%20Component%20Object%20Reference) (OtherBodyIndex :type Integer) (bFromSweep :type Boolean) (SweepResult :type Hit%20Result%20Structure%20%28by%20ref%29))
  (bind _asthird_person_character (Utilities|Casting|CastToThirdPersonCharacter OtherActor))
  (Variables|Default|SetScore (Variables|/Game/ThirdPersonBP/Blueprints/ThirdPersonCharacter.ThirdPersonCharacter_C|GetKillcount _asthird_person_character))
  (if (>= (Variables|/Game/ThirdPersonBP/Blueprints/ThirdPersonCharacter.ThirdPersonCharacter_C|GetKillcount _asthird_person_character) 200)
    (bind _asthird_person_character_2 (Utilities|Casting|CastToThirdPersonCharacter OtherActor))
    (Variables|Default|SetArme (Variables|/Game/ThirdPersonBP/Blueprints/ThirdPersonCharacter.ThirdPersonCharacter_C|GetEquippedWeapon _asthird_person_character_2))
    (if (== (Variables|/Game/AK/Ak_base.Ak_base_C|GetMaxAmmo (Variables|Default|GetArme)) 360)
      (Development|PrintString "Chargeurs pleins")
      (else
        (if (>= (+ (Variables|Default|GetPickupAmmo) (Variables|/Game/AK/Ak_base.Ak_base_C|GetMaxAmmo (Variables|Default|GetArme))) 360)
          (Variables|/Game/AK/Ak_base.Ak_base_C|SetMaxAmmo (Variables|Default|GetArme) 360)
          (Audio|PlaySoundatLocation "/Game/Sound/377551__bunny-clark__ar-reload.377551__bunny-clark__ar-reload" "0, 0, 0")
          (else
            (Variables|/Game/AK/Ak_base.Ak_base_C|SetMaxAmmo (Variables|Default|GetArme) (+ (Variables|Default|GetPickupAmmo) (Variables|/Game/AK/Ak_base.Ak_base_C|GetMaxAmmo (Variables|Default|GetArme))))))
        (Variables|/Game/ThirdPersonBP/Blueprints/ThirdPersonCharacter.ThirdPersonCharacter_C|SetKillcount _asthird_person_character_2 (- (Variables|Default|GetScore) 200))))
    (else
      (Development|PrintString "Pas assez de point"))))

(event EventBeginPlay
  (|CallParentFunction))

(fn ConstructionScript
  (|CallParentFunction))